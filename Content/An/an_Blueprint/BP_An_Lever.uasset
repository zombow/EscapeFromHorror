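; BP_An_Lever is a lever actor that sets an OpenDoor flag when the player activates it with the G key.
; Box overlap events track whether BP_An_Player is inside, and G press and release track the held key.
; Both flags are checked only when overlap begins, so G must already be held on entry.
; OpenDoor is never reset, and this graph contains no door movement.
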(event OnComponentBeginOverlap(Box)
  (params (OverlappedComponent :type Primitive%20Component%20Object%20Reference) (OtherActor :type Actor%20Object%20Reference) (OtherComp :type Primitive%20Component%20Object%20Reference) (OtherBodyIndex :type Integer) (bFromSweep :type Boolean) (SweepResult :type Hit%20Result%20Structure%20%28by%20ref%29))
  (Utilities|Casting|CastToBP_An_Player OtherActor)
  (Variables|Default|SetOnTop? true)
  (if (and (Variables|Default|GetpressG?) (Variables|Default|GetOnTop?))
    (Variables|Default|SetOpenDoor true)))

(event OnComponentEndOverlap(Box)
  (params (OverlappedComponent :type Primitive%20Component%20Object%20Reference) (OtherActor :type Actor%20Object%20Reference) (OtherComp :type Primitive%20Component%20Object%20Reference) (OtherBodyIndex :type Integer))
  (Utilities|Casting|CastToBP_An_Player OtherActor)
  (Variables|Default|SetOnTop? false))

(event EventBeginPlay)

(event Collision|EventActorBeginOverlap
  (params (OtherActor :type Actor%20Object%20Reference)))

(event EventTick
  (params (DeltaSeconds :type Float%20%28single-precision%29)))

(event Input|KeyboardEvents|G
  (params (Key :type Key%20Structure :default "None"))
  (:Pressed
    (Variables|Default|SetpressG? true))
  (:Released
    (Variables|Default|SetpressG? false)))

(fn ConstructionScript)