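; Pushable object that BP_An_Player can shove along while inside either of its two trigger boxes.
; Player overlap turns on physics simulation for the Move component; leaving, or another actor entering, turns it off.
; While active, Tick treats grounded Y-axis velocity as pushing, setting IsPushing on the player and ABP_An_Player and lowering walk speed.
; Leaving restores normal speed and clears the animation flag.
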(event OnComponentBeginOverlap(Box)
  (params (OverlappedComponent :type Primitive%20Component%20Object%20Reference) (OtherActor :type Actor%20Object%20Reference) (OtherComp :type Primitive%20Component%20Object%20Reference) (OtherBodyIndex :type Integer) (bFromSweep :type Boolean) (SweepResult :type Hit%20Result%20Structure%20%28by%20ref%29))
  (if (or (== (stale OnComponentBeginOverlap(Box1) OtherActor) (Variables|Default|GetPlayer)) (== OtherActor (Variables|Default|GetPlayer)))
    (bind _output_get (Variables|Default|SetTick true))
    (CallFunction|ChangePhysics _output_get)
    (else
      (bind _output_get_2 (Variables|Default|SetTick false))
      (CallFunction|ChangePhysics _output_get_2))))

(event OnComponentEndOverlap(Box)
  (params (OverlappedComponent :type Primitive%20Component%20Object%20Reference) (OtherActor :type Actor%20Object%20Reference) (OtherComp :type Primitive%20Component%20Object%20Reference) (OtherBodyIndex :type Integer))
  (if (or (== (stale OnComponentEndOverlap(Box1) OtherActor) (Variables|Default|GetPlayer)) (== OtherActor (Variables|Default|GetPlayer)))
    (bind _output_get (Variables|Default|SetTick false))
    (CallFunction|ChangePhysics _output_get)
    (Variables|/Script/Engine.CharacterMovementComponent|SetMaxWalkSpeed (Variables|/Script/Engine.Character|GetCharacterMovement (Variables|Default|GetPlayer)) 1.5e+02)
    (bind _asabp_an_player (Utilities|Casting|CastToABP_An_Player (Components|SkeletalMesh|GetAnimInstance (Variables|/Script/Engine.Character|GetMesh (Variables|Default|GetPlayer)))))
    (Variables|/Game/An/an_Blueprint/ABP_An_Player.ABP_An_Player_C|SetisPushing _asabp_an_player false)))

(event OnComponentBeginOverlap(Box1)
  (params (OverlappedComponent :type Primitive%20Component%20Object%20Reference) (OtherActor :type Actor%20Object%20Reference) (OtherComp :type Primitive%20Component%20Object%20Reference) (OtherBodyIndex :type Integer) (bFromSweep :type Boolean) (SweepResult :type Hit%20Result%20Structure%20%28by%20ref%29))
  (if (or (== OtherActor (Variables|Default|GetPlayer)) (== (stale OnComponentBeginOverlap(Box) OtherActor) (Variables|Default|GetPlayer)))
    (bind _output_get (Variables|Default|SetTick true))
    (CallFunction|ChangePhysics _output_get)
    (else
      (bind _output_get_2 (Variables|Default|SetTick false))
      (CallFunction|ChangePhysics _output_get_2))))

(event OnComponentEndOverlap(Box1)
  (params (OverlappedComponent :type Primitive%20Component%20Object%20Reference) (OtherActor :type Actor%20Object%20Reference) (OtherComp :type Primitive%20Component%20Object%20Reference) (OtherBodyIndex :type Integer))
  (if (or (== OtherActor (Variables|Default|GetPlayer)) (== (stale OnComponentEndOverlap(Box) OtherActor) (Variables|Default|GetPlayer)))
    (bind _output_get (Variables|Default|SetTick false))
    (CallFunction|ChangePhysics _output_get)
    (Variables|/Script/Engine.CharacterMovementComponent|SetMaxWalkSpeed (Variables|/Script/Engine.Character|GetCharacterMovement (Variables|Default|GetPlayer)) 1.5e+02)
    (bind _asabp_an_player (Utilities|Casting|CastToABP_An_Player (Components|SkeletalMesh|GetAnimInstance (Variables|/Script/Engine.Character|GetMesh (Variables|Default|GetPlayer)))))
    (Variables|/Game/An/an_Blueprint/ABP_An_Player.ABP_An_Player_C|SetisPushing _asabp_an_player false)))

(event EventBeginPlay
  (bind _asbp_an_player (Utilities|Casting|CastToBP_An_Player (Game|GetPlayerCharacter 0)))
  (Variables|Default|SetPlayer _asbp_an_player))

(event Collision|EventActorBeginOverlap
  (params (OtherActor :type Actor%20Object%20Reference)))

(event EventTick
  (params (DeltaSeconds :type Float%20%28single-precision%29))
  (bind _player (Variables|Default|GetPlayer))
  (bind _charactermovement (Variables|/Script/Engine.Character|GetCharacterMovement _player))
  (bind _mesh (Variables|/Script/Engine.Character|GetMesh _player))
  (bind _returnvalue (Components|SkeletalMesh|GetAnimInstance _mesh))
  (if (Variables|Default|GetTick)
    (if (and (!= (.Y (Math|Vector|BreakVector (Variables|/Script/Engine.MovementComponent|GetVelocity (Variables|/Script/Engine.Character|GetCharacterMovement (Variables|Default|GetPlayer))))) 0.0) (not (AI|Components|NavMovement|IsFalling (Variables|/Script/Engine.Character|GetCharacterMovement (Variables|Default|GetPlayer)))))
      (bind _output_get (Variables|/Game/An/an_Blueprint/BP_An_Player.BP_An_Player_C|SetIsPushing _player true))
      (bind _asabp_an_player (Utilities|Casting|CastToABP_An_Player _returnvalue))
      (Variables|/Game/An/an_Blueprint/ABP_An_Player.ABP_An_Player_C|SetisPushing _asabp_an_player _output_get)
      (Variables|/Script/Engine.CharacterMovementComponent|SetMaxWalkSpeed _charactermovement 9e+01)
      (else
        (bind _output_get_2 (Variables|/Game/An/an_Blueprint/BP_An_Player.BP_An_Player_C|SetIsPushing _player false))
        (bind _asabp_an_player_2 (Utilities|Casting|CastToABP_An_Player _returnvalue))
        (Variables|/Game/An/an_Blueprint/ABP_An_Player.ABP_An_Player_C|SetisPushing _asabp_an_player_2 _output_get_2)
        (Variables|/Script/Engine.CharacterMovementComponent|SetMaxWalkSpeed _charactermovement 1.5e+02)))))

(fn ConstructionScript)

(fn ChangePhysics
  (params (Simulate :type Boolean))
  (Physics|SetSimulatePhysics (Variables|Default|GetMove) Simulate))